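; HUD Blueprint meant to draw circular stamina and health bars for the player character, though its drawing chain is disconnected and DrawHUD is empty.
; Tick only sets a colour variable: green when cached Stamina exceeds a small threshold, grey otherwise.
; The unreachable chain would refresh that cache and draw CircleHealthBar_Mat dynamic instances, filled by current-to-max ratios from PlayerCharater_Bp, with health in red.
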(event `self.ReceiveDrawHUD`
  (params (SizeX :type Integer) (SizeY :type Integer)))

(event `self.ReceiveBeginPlay`)

(event `self.ReceiveTick`
  (params (DeltaSeconds :type "Float (single-precision)"))
  (if (> (`self.Stamina`) 5.0)
    (set `self.Value` (struct :`G` 0.494792 :`B` 0.054399 :`A` 1.0))
    (else
      (set `self.Value` (struct :`R` 0.15625 :`G` 0.15625 :`B` 0.15625 :`A` 1.0)))))

(fn `UserConstructionScript`)