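; Modular party monster character Blueprint that builds a randomized look from separate skeletal mesh parts when play begins.
; On BeginPlay, gloves, body parts, eyes, mouths, noses, tails and head parts follow the main skeletal mesh through Set Master Pose Component, sharing its pose.
; RandomMeshes then gives the base body and each part a random mesh from its own array, reinitializing the pose.
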(event `RandomMeshes`
  (`SkinnedMeshComponent.SetSkinnedAssetAndUpdate` (`self.SkeletalMeshComponent`) (`KismetArrayLibrary.Array_Random` (`self.BodyArray`)) true)
  (`SkinnedMeshComponent.SetSkinnedAssetAndUpdate` (`self.Bodyparts`) (`KismetArrayLibrary.Array_Random` (`self.BodyPartArray`)) true)
  (`SkinnedMeshComponent.SetSkinnedAssetAndUpdate` (`self.Mouths`) (`KismetArrayLibrary.Array_Random` (`self.MouthArray`)) true)
  (`SkinnedMeshComponent.SetSkinnedAssetAndUpdate` (`self.Gloves`) (`KismetArrayLibrary.Array_Random` (`self.GlovesArray`)) true)
  (`SkinnedMeshComponent.SetSkinnedAssetAndUpdate` (`self.Noses`) (`KismetArrayLibrary.Array_Random` (`self.NosesArrayMale`)) true)
  (`SkinnedMeshComponent.SetSkinnedAssetAndUpdate` (`self.Tails`) (`KismetArrayLibrary.Array_Random` (`self.TailsArray`)) true)
  (`SkinnedMeshComponent.SetSkinnedAssetAndUpdate` (`self.Headparts`) (`KismetArrayLibrary.Array_Random` (`self.HeadpartsArray`)) true)
  (`SkinnedMeshComponent.SetSkinnedAssetAndUpdate` (`self.Eyes`) (`KismetArrayLibrary.Array_Random` (`self.EyesArray`)) true))

(event `self.ReceiveBeginPlay`
  (`SkinnedMeshComponent.SetLeaderPoseComponent` (`self.Gloves`) (`self.SkeletalMeshComponent`) false)
  (`SkinnedMeshComponent.SetLeaderPoseComponent` (`self.Bodyparts`) (`self.SkeletalMeshComponent`) false)
  (`SkinnedMeshComponent.SetLeaderPoseComponent` (`self.Eyes`) (`self.SkeletalMeshComponent`) false)
  (`SkinnedMeshComponent.SetLeaderPoseComponent` (`self.Mouths`) (`self.SkeletalMeshComponent`) false)
  (`SkinnedMeshComponent.SetLeaderPoseComponent` (`self.Noses`) (`self.SkeletalMeshComponent`) false)
  (`SkinnedMeshComponent.SetLeaderPoseComponent` (`self.Tails`) (`self.SkeletalMeshComponent`) false)
  (`SkinnedMeshComponent.SetLeaderPoseComponent` (`self.Headparts`) (`self.SkeletalMeshComponent`) false)
  (`self.RandomMeshes`))

(fn `UserConstructionScript`)