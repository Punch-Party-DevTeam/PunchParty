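; HUD Blueprint that draws circular stamina and health gauges for the player character.
; DrawHUD creates two CircleHealthBar_Mat dynamic instances on every call, setting color and fill ratio from PlayerCharacter_Bp before drawing them at fixed screen positions.
; Tick switches the stamina color between green and grey using a threshold on the Stamina value cached during DrawHUD, while health is always red.
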(event `self.ReceiveBeginPlay`)

(event `self.ReceiveDrawHUD`
  (params (SizeX :type Integer) (SizeY :type Integer))
  (bind _returnvalue (`KismetMaterialLibrary.CreateDynamicMaterialInstance` "/Game/Materials/CircleHealthBar_Mat.CircleHealthBar_Mat"))
  (`MaterialInstanceDynamic.SetVectorParameterValue` _returnvalue "Color" (`self.Value`))
  (bind _asplayer_character_bp (cast `/Game/ThirdPersonBP/Blueprints/PlayerCharacter_Bp` (`GameplayStatics.GetPlayerCharacter` 0)))
  (bind _stamina (`/Game/ThirdPersonBP/Blueprints/PlayerCharacter_Bp.Stamina` _asplayer_character_bp))
  (`MaterialInstanceDynamic.SetScalarParameterValue` _returnvalue "Decimal" (/ _stamina (`/Game/ThirdPersonBP/Blueprints/PlayerCharacter_Bp.MaxStamina` _asplayer_character_bp)))
  (set `self.Stamina` _stamina)
  (`self.DrawMaterialSimple` _returnvalue 100.0 100.0 100.0 100.0)
  (bind _returnvalue_2 (`KismetMaterialLibrary.CreateDynamicMaterialInstance` "/Game/Materials/CircleHealthBar_Mat.CircleHealthBar_Mat"))
  (`MaterialInstanceDynamic.SetVectorParameterValue` _returnvalue_2 "Color" (struct :`R` 1.0 :`A` 1.0))
  (bind _asplayer_character_bp_2 (cast `/Game/ThirdPersonBP/Blueprints/PlayerCharacter_Bp` (`GameplayStatics.GetPlayerCharacter` 0)))
  (`MaterialInstanceDynamic.SetScalarParameterValue` _returnvalue_2 "Decimal" (/ (`/Game/ThirdPersonBP/Blueprints/PlayerCharacter_Bp.Health` _asplayer_character_bp_2) (`/Game/ThirdPersonBP/Blueprints/PlayerCharacter_Bp.MaxHealth` _asplayer_character_bp_2)))
  (`self.DrawMaterialSimple` _returnvalue_2 200.0 200.0 100.0 100.0))

(event `self.ReceiveTick`
  (params (DeltaSeconds :type "Float (single-precision)"))
  (if (> (`self.Stamina`) 5.0)
    (set `self.Value` (struct :`G` 0.494792 :`B` 0.054399 :`A` 1.0))
    (else
      (set `self.Value` (struct :`R` 0.15625 :`G` 0.15625 :`B` 0.15625 :`A` 1.0)))))

(fn `UserConstructionScript`)